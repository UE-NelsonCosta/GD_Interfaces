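; BP_InteractingPawn is a pawn that lets the player interact with whatever sits at the screen center on a left click.
; CalculateHitObject deprojects the viewport center to a world ray and line traces it on Visibility up to RayRange, leaving persistent debug lines.
; On a hit, ProcessInteraction sends CanInteractMessage to the hit actor and, if it returns true, calls InteractMessage on it.
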(event `Key|LeftMouseButton`
  (params (Key :type "Key Structure"))
  (:`Pressed`
    (bind (_hitresult _hitstate) (`self.CalculateHitObject`))
    (if _hitstate
      (`self.ProcessInteraction` _hitresult))))

(fn `CalculateHitObject`
  (returns (HitResult :type "HitResult Structure") (HitState :type Boolean))
  (bind _asplayer_controller (cast `PlayerController` (`self.GetController`)))
  (bind (_worldposition _worlddirection) (`GameplayStatics.DeprojectScreenToWorld` _asplayer_controller (/ (`WidgetLayoutLibrary.GetViewportSize`) 2.0)))
  (bind (_outhit _returnvalue) (`KismetSystemLibrary.LineTraceSingle` :`Start` _worldposition :`End` (+ _worldposition (* _worlddirection (`self.RayRange`))) :`TraceChannel` "TraceTypeQuery1" :`DrawDebugType` "Persistent"))
  (return _outhit _returnvalue))

(fn `ProcessInteraction`
  (params (HitResult :type "HitResult Structure"))
  (bind (_bblockinghit _binitialoverlap _time _distance _location _impactpoint _normal _impactnormal _physmat _hitactor) (`GameplayStatics.BreakHitResult` HitResult))
  (bind _state (message `/Game/BP_IInteractable.CanInteract` _hitactor null))
  (if _state
    (message `/Game/BP_IInteractable.Interact` _hitactor null)))

(fn `UserConstructionScript`)